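; Drone actor that flies along the spline of a MySplineOLD actor found in the level.
; On BeginPlay it caches that actor and starts a timeline with a play rate of one over TimeToCompleteCycle.
; Each update maps the timeline's MoveTrack value to a distance along the spline and sets the drone's world location and rotation from that point.
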(event Custom|FlyDrone
  (bind _mysplineref (Variables|Default|GetmysplineRef))
  (bind _myspline (Variables|/Game/Blueprints/mySplineOLD.mySplineOLD_C|GetmySpline _mysplineref))
  (Components|Timeline|SetPlayRate (Variables|Default|GetDroneTimeline) (/ 1.0 (Variables|Default|GettimeToCompleteCycle)))
  (bind _movetrack (Timeline|DroneTimeline Play)
    (:Update
      (Transformation|SetActorTransform (Math|Transform|MakeTransform (Spline|GetLocationatDistanceAlongSpline _myspline (Math|Float|Lerp 0.0 (Spline|GetSplineLength (Variables|/Game/Blueprints/mySplineOLD.mySplineOLD_C|GetmySpline (Variables|Default|GetmysplineRef))) _movetrack) "World") (Spline|GetRotationatDistanceAlongSpline _myspline (Math|Float|Lerp 0.0 (Spline|GetSplineLength (Variables|/Game/Blueprints/mySplineOLD.mySplineOLD_C|GetmySpline (Variables|Default|GetmysplineRef))) _movetrack) "World") "1.000000,1.000000,1.000000")))))

(event EventBeginPlay
  (bind _returnvalue (Actor|GetActorOfClass "/Game/Blueprints/mySplineOLD.mySplineOLD_C"))
  (Variables|Default|SetmysplineRef _returnvalue)
  (CallFunction|FlyDrone))

(fn ConstructionScript)