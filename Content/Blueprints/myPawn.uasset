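; Player pawn that lets the user lay out a spline path with the mouse and then launch a drone along with the yacht actor's FlyDrone.
; Left mouse release toggles drawing via FlipFlop; switching it off calls FlyDrone on the BP_myYatch found at BeginPlay.
; While drawing, a delayed Tick traces from the cursor into the world and appends each hit location as a point on Bp_mySpline's DynamicSpline.
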(event EventBeginPlay
  (Variables|/Script/Engine.PlayerController|SetbShowMouseCursor (Game|GetPlayerController 0) true)
  (bind _returnvalue (Actor|GetActorOfClass "/Game/Blueprints/bp_mySpline.bp_mySpline_C"))
  (Variables|Default|SetmySpline _returnvalue)
  (bind _returnvalue_2 (Actor|GetActorOfClass "/Game/Blueprints/BP_myYatch.BP_myYatch_C"))
  (Variables|Default|SetmyYatchRef _returnvalue_2))

(event EventTick
  (params (DeltaSeconds :type Float%20%28single-precision%29))
  (bind _returnvalue (Game|GetPlayerController 0))
  (bind _myspline (Variables|Default|GetmySpline))
  (bind (_locationx _locationy) (Game|Player|GetMousePosition _returnvalue))
  (bind _dynamicspline (Variables|/Game/Blueprints/bp_mySpline.bp_mySpline_C|GetdynamicSpline _myspline))
  (bind (_worldlocation _worlddirection) (Class|PlayerController|DeprojectScreenPositiontoWorld _returnvalue _locationx _locationy))
  (Utilities|FlowControl|Delay 1.0)
  (if (Variables|Default|GetmouseClicked?)
    (bind _outhit (Collision|LineTraceByChannel _worldlocation (+ _worldlocation (* _worlddirection 1.5e+03)) "TraceTypeQuery1" false 0 "ForDuration"))
    (bind _output_get (Variables|Default|SetlocationToDrawSplinePoints (.location _outhit)))
    (Development|PrintString (Utilities|String|ToString(Integer) (Spline|GetNumberOfSplinePoints _dynamicspline)))
    (Spline|AddSplinePoint _dynamicspline _output_get "World" true)))

(event Input|MouseEvents|LeftMouseButton
  (params (Key :type Key%20Structure :default "None"))
  (:Released
    (Utilities|FlowControl|FlipFlop
      (:A
        (Variables|Default|SetmouseClicked? true))
      (:B
        (Variables|Default|SetmouseClicked? false)
        (Default|FlyDrone (Variables|Default|GetmyYatchRef))))))

(fn ConstructionScript)