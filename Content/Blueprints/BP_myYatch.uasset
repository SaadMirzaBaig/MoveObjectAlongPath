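; Yacht actor that travels along the spline of a Bp_mySpline actor in the level.
; BeginPlay finds and caches that spline actor.
; The FlyDrone event plays a timeline with its rate set to the inverse of TimeToCompleteCycle.
; Each update maps the MoveTrack alpha to a distance along DynamicSpline and sets the yacht's world location and rotation from that point.
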(event Custom|FlyDrone
  (bind _mysplineref (Variables|Default|GetmySplineRef))
  (bind _dynamicspline (Variables|/Game/Blueprints/bp_mySpline.bp_mySpline_C|GetdynamicSpline _mysplineref))
  (Components|Timeline|SetPlayRate (Variables|Default|GetyatchTimeline) (/ 1.0 (Variables|Default|GettimeToCompleteCycle)))
  (bind _movetrack (Timeline|yatchTimeline Play)
    (:Update
      (Transformation|SetActorTransform (Math|Transform|MakeTransform (Spline|GetLocationatDistanceAlongSpline _dynamicspline (Math|Float|Lerp 0.0 (Spline|GetSplineLength (Variables|/Game/Blueprints/bp_mySpline.bp_mySpline_C|GetdynamicSpline (Variables|Default|GetmySplineRef))) _movetrack) "World") (Spline|GetRotationatDistanceAlongSpline _dynamicspline (Math|Float|Lerp 0.0 (Spline|GetSplineLength (Variables|/Game/Blueprints/bp_mySpline.bp_mySpline_C|GetdynamicSpline (Variables|Default|GetmySplineRef))) _movetrack) "World") "1.000000,1.000000,1.000000")))))

(event EventBeginPlay
  (bind _returnvalue (Actor|GetActorOfClass "/Game/Blueprints/bp_mySpline.bp_mySpline_C"))
  (Variables|Default|SetmySplineRef _returnvalue))

(fn ConstructionScript)